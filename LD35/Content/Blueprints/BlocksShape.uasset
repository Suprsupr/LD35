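; BlocksShape is a Blueprint that spawns a randomized cluster of blocks at BeginPlay.
; CreateShapeLayer walks a 3x4 grid spaced by CubeWidth, giving cells on two edges a low chance of a BlockVideo_Blueprint and the rest a higher chance of a Block_Blueprint.
; Each block gets random height, pitch, yaw and uniform scale.
; Positions ignore the actor's location, and the BlockLocationZ input is unused.
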(event EventBeginPlay
  (CallFunction|CreateShapeLayer (Math|Vector|MakeVector 0.0 0.0 (Variables|Default|GetlastLayerZ))))

(fn ConstructionScript)

(fn CreateShapeLayer
  (params (blockLocationZ :type Vector))
  (bind _returnvalue (Math|Random|RandomFloatinRange 0.0 2e+01))
  (bind _cubewidth (Variables|Default|GetcubeWidth))
  (for _index (range 0 2)
    (for _index_2 (range 0 3)
      (if (or (== _index 2) (== _index_2 0))
        (if (<= (Math|Random|RandomInteger 100) 16)
          (Game|SpawnActorfromClass "/Game/Blueprints/blockVideo_Blueprint.BlockVideo_Blueprint_C" (Math|Transform|MakeTransform (Math|Vector|MakeVector (* (Math|Conversions|ToFloat(Integer) _index_2) _cubewidth) (* (Math|Conversions|ToFloat(Integer) _index) _cubewidth) (Math|Random|RandomFloatinRange 0.0 5e+02)) (Math|Rotator|MakeRotator 0.0 _returnvalue _returnvalue) (Math|Conversions|ToVector(Float) (Math|Random|RandomFloatinRange 1.0 4.0))) "Undefined" 0 0))
        (elif (<= (Math|Random|RandomInteger 100) 60)
          (Game|SpawnActorfromClass "/Game/Blueprints/Block_Blueprint.Block_Blueprint_C" (Math|Transform|MakeTransform (Math|Vector|MakeVector (* (Math|Conversions|ToFloat(Integer) _index_2) _cubewidth) (* (Math|Conversions|ToFloat(Integer) _index) _cubewidth) (Math|Random|RandomFloatinRange 0.0 5e+02)) (Math|Rotator|MakeRotator 0.0 _returnvalue _returnvalue) (Math|Conversions|ToVector(Float) (Math|Random|RandomFloatinRange 1.0 4.0))) "Undefined" 0 0))))))