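; Level generator that scatters fourteen randomized tree-like clusters of blocks across the map at BeginPlay.
; Each CreateTree anchors a cluster at the hit location of a random downward, slanted line trace.
; CreateShape probabilistically spawns a jittered grid of Block actors, with rarer BlockVideo actors on two edges.
; CreateShapeBranches adds a higher layer of blocks, reusing the cluster's random material and base size.
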(event OnClicked(trigger)
  (params (TouchedComponent :type Primitive%20Component%20Object%20Reference)))

(event EventTick
  (params (DeltaSeconds :type Float%20%28single-precision%29)))

(event EventBeginPlay
  (Utilities|FlowControl|Sequence
    (:then_0
      (CallFunction|CreateTree))
    (:then_1
      (CallFunction|CreateTree))
    (:then_2
      (CallFunction|CreateTree))
    (:then_3
      (CallFunction|CreateTree))
    (:then_4
      (CallFunction|CreateTree))
    (:then_5
      (CallFunction|CreateTree))
    (:then_6
      (CallFunction|CreateTree))
    (:then_7
      (CallFunction|CreateTree))
    (:then_8
      (CallFunction|CreateTree))
    (:then_9
      (CallFunction|CreateTree))
    (:then_10
      (CallFunction|CreateTree))
    (:then_11
      (CallFunction|CreateTree))
    (:then_12
      (CallFunction|CreateTree))
    (:then_13
      (CallFunction|CreateTree))))

(fn ConstructionScript)

(fn CreateShape
  (params (blockLocation :type Vector) (shapeSize :type Vector))
  (bind _cubewidth (Variables|Default|GetcubeWidth))
  (Variables|Default|SetrandomMatNum (Math|Random|RandomInteger 12))
  (for _index (range 0 2)
    (for _index_2 (range 0 3)
      (if (or (== _index 2) (== _index_2 0))
        (if (<= (Math|Random|RandomInteger 100) 16)
          (Game|SpawnActorfromClass "/Game/Blueprints/blockVideo_Blueprint.BlockVideo_Blueprint_C" (Math|Transform|MakeTransform (+ blockLocation (Math|Vector|MakeVector (* (Math|Conversions|ToFloat(Integer) _index_2) (+ _cubewidth (Math|Random|RandomFloatinRange 0.0 1.6e+02))) (* (Math|Conversions|ToFloat(Integer) _index) _cubewidth) (Math|Random|RandomFloatinRange -2e+01 7e+02))) (Math|Rotator|MakeRotator 0.0 (Math|Random|RandomFloatinRange 0.0 2e+01) (Math|Random|RandomFloatinRange 0.0 4e+01)) (+ shapeSize (Math|Conversions|ToVector(Float) (Math|Random|RandomFloatinRange 1.5 4.0)))) "Undefined" 0 0))
        (elif (<= (Math|Random|RandomInteger 100) 60)
          (bind _returnvalue (Game|SpawnActorfromClass "/Game/Blueprints/Block_Blueprint.Block_Blueprint_C" (Math|Transform|MakeTransform (+ blockLocation (Math|Vector|MakeVector (* (Math|Conversions|ToFloat(Integer) _index_2) (+ _cubewidth (Math|Random|RandomFloatinRange 0.0 1.6e+02))) (* (Math|Conversions|ToFloat(Integer) _index) _cubewidth) (Math|Random|RandomFloatinRange -2e+01 7e+02))) (Math|Rotator|MakeRotator 0.0 (Math|Random|RandomFloatinRange 0.0 2e+01) (Math|Random|RandomFloatinRange 0.0 4e+01)) (+ shapeSize (Math|Conversions|ToVector(Float) (Math|Random|RandomFloatinRange 1.5 4.0)))) "Undefined" 0 0))
          (Rendering|Material|SetMaterial (Variables|/Script/Engine.StaticMeshActor|GetStaticMeshComponent _returnvalue) 0 (Utilities|Array|Get(acopy) (Variables|Default|Getmat) (Variables|Default|GetrandomMatNum))))))))

(fn LineTracing
  (bind _returnvalue (Math|Random|RandomFloatinRange -1.4e+04 1.4e+04))
  (bind _returnvalue_2 (Math|Random|RandomFloatinRange -1.4e+04 1.4e+04))
  (Variables|Default|SetstartLineTracingPoint (Math|Vector|MakeVector _returnvalue_2 _returnvalue 2e+03))
  (Variables|Default|SetendLineTracingPoint (Math|Vector|MakeVector _returnvalue_2 _returnvalue -1e+03))
  (bind _outhit (Collision|LineTraceByChannel (Variables|Default|GetstartLineTracingPoint) (Variables|Default|GetendLineTracingPoint) "TraceTypeQuery1" false 0 "None"))
  (return (.Location (Collision|BreakHitResult _outhit))))

(fn CreateShapeBranches
  (params (BlockLocation :type Vector) (shapeBrancheSize :type Vector))
  (bind _returnvalue (Math|Random|RandomFloatinRange 0.6 1.5))
  (bind _cubewidth (Variables|Default|GetcubeWidth))
  (bind _returnvalue_2 (Math|Conversions|ToVector(Float) _returnvalue))
  (for _index (range 0 2)
    (for _index_2 (range 0 2)
      (if (<= (Math|Random|RandomInteger 100) 60)
        (bind _returnvalue_3 (Game|SpawnActorfromClass "/Game/Blueprints/Block_Blueprint.Block_Blueprint_C" (Math|Transform|MakeTransform (+ BlockLocation (Math|Vector|MakeVector (* (Math|Conversions|ToFloat(Integer) _index_2) (+ _cubewidth (Math|Random|RandomFloatinRange 0.0 1e+02))) (* (Math|Conversions|ToFloat(Integer) _index) _cubewidth) (Math|Random|RandomFloatinRange 9e+02 1.3e+03))) (Math|Rotator|MakeRotator 0.0 (Math|Random|RandomFloatinRange 0.0 2e+01) (Math|Random|RandomFloatinRange 0.0 1.8e+02)) (/ (+ shapeBrancheSize _returnvalue_2) _returnvalue_2)) "Undefined" 0 0))
        (Rendering|Material|SetMaterial (Variables|/Script/Engine.StaticMeshActor|GetStaticMeshComponent _returnvalue_3) 0 (Utilities|Array|Get(acopy) (Variables|Default|Getmat) (Variables|Default|GetrandomMatNum)))))))

(fn CreateTree
  (bind _returnvalue (Math|Random|RandomFloatinRange -1.0 5.0))
  (bind _location (CallFunction|LineTracing))
  (bind _output_get (Variables|Default|SetshapeSize (Math|Vector|MakeVector _returnvalue _returnvalue _returnvalue)))
  (CallFunction|CreateShape _location _output_get)
  (CallFunction|CreateShapeBranches _location _output_get))