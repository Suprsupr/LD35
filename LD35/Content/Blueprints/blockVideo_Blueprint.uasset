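; Block actor that shows a random video material on its static mesh and plays audio when play begins.
; BeginPlay starts RandomAudio, applies one of seven VideoMat entries and plays one of seven MediaPlayers.
; Material and player are picked by separate random rolls, so they can differ.
; The Trigger click event is empty, and a node setting the Simple2Sided material is left unconnected.
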(event OnClicked(trigger)
  (params (TouchedComponent :type Primitive%20Component%20Object%20Reference)))

(event EventBeginPlay
  (bind _returnvalue (Math|Random|RandomInteger 7))
  (Audio|Components|Audio|Play (Variables|Default|GetRandomAudio) 0.0)
  (Rendering|Material|SetMaterial (Variables|Debug|GetStaticMeshComponent) 0 (Utilities|Array|Get(acopy) (Variables|Default|GetvideoMat) _returnvalue))
  (Media|MediaPlayer|Play (Utilities|Array|Get(acopy) (Variables|Default|GetmediaPlayers) _returnvalue) :!class /Script/MediaAssets.MediaPlayer))

(fn ConstructionScript)